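; Ticket barrier for the VR train game that swings its two doors open when a ticket is inserted.
; Either insert trigger destroys the ticket, clears the WalletManager ticket flag, then after a delay spawns a replacement at its paired spawn point.
; A timeline rotates the doors and toggles blocking collision, reversing after a timed hold to close and re-arm.
; The Broken flag presets the barrier open without collision.
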(event OnComponentBeginOverlap(TicketInsert2)
  (params (OverlappedComponent :type Primitive%20Component%20Object%20Reference) (OtherActor :type Actor%20Object%20Reference) (OtherComp :type Primitive%20Component%20Object%20Reference) (OtherBodyIndex :type Integer) (bFromSweep :type Boolean) (SweepResult :type Hit%20Result%20Structure%20%28by%20ref%29))
  (bind _asticket (Utilities|Casting|CastToTicket OtherActor))
  (if (not (Variables|Default|GetTicketActive?))
    (Actor|DestroyActor _asticket)
    (bind _outactors (Actor|GetAllActorsOfClass "/Game/VRTrain/BPs/interactions/WalletManager.WalletManager_C"))
    (Variables|/Game/VRTrain/BPs/interactions/WalletManager.WalletManager_C|SetTicket? (Utilities|Array|Get(acopy) _outactors) false)
    (Utilities|FlowControl|Delay 2.0)
    (Variables|Default|SetTicketActive? true)
    (bind _returnvalue (Game|SpawnActorfromClass "/Game/VRTrain/BPs/interactions/Ticket.Ticket_C" (Transformation|GetWorldTransform (Variables|Default|Getspawn2)) "Undefined" 0 0))
    (Transformation|SetActorRelativeScale3D _returnvalue "0.200000,0.200000,0.200000")
    (CallFunction|OpenBarriers)))

(event OnComponentBeginOverlap(TicketInsert)
  (params (OverlappedComponent :type Primitive%20Component%20Object%20Reference) (OtherActor :type Actor%20Object%20Reference) (OtherComp :type Primitive%20Component%20Object%20Reference) (OtherBodyIndex :type Integer) (bFromSweep :type Boolean) (SweepResult :type Hit%20Result%20Structure%20%28by%20ref%29))
  (bind _asticket (Utilities|Casting|CastToTicket OtherActor))
  (if (not (Variables|Default|GetTicketActive?))
    (Actor|DestroyActor _asticket)
    (bind _outactors (Actor|GetAllActorsOfClass "/Game/VRTrain/BPs/interactions/WalletManager.WalletManager_C"))
    (Variables|/Game/VRTrain/BPs/interactions/WalletManager.WalletManager_C|SetTicket? (Utilities|Array|Get(acopy) _outactors) false)
    (Utilities|FlowControl|Delay 2.0)
    (Variables|Default|SetTicketActive? true)
    (bind _returnvalue (Game|SpawnActorfromClass "/Game/VRTrain/BPs/interactions/Ticket.Ticket_C" (Transformation|GetWorldTransform (Variables|Default|Getspawn1)) "Undefined" 0 0))
    (Transformation|SetActorRelativeScale3D _returnvalue "0.200000,0.200000,0.200000")
    (CallFunction|OpenBarriers)))

(event Custom|open%20barriers
  (bind _cube (Variables|Default|GetCube))
  ;[1 1 1] Open and close Gates
  (Variables|Default|SetOpen? true)
  (bind _opentrack (Timeline|OpenBarriers Play)
    (:Update
      (Transformation|SetRelativeRotation (Variables|Default|GetBarrier_Door) (Math|Rotator|Lerp(Rotator) "0, 0, 0" "0,90.000000, 0" _opentrack) false false)
      (Transformation|SetRelativeRotation (Variables|Default|GetBarrier_Door1) (Math|Rotator|Lerp(Rotator) "0,180.000000, 0" "0,270.000000, 0" _opentrack) false false))
    (:Finished
      (if (Variables|Default|GetOpen?)
        (Collision|SetCollisionEnabled _cube "NoCollision")
        (Utilities|FlowControl|Delay 12.0)
        (CallFunction|CloseBarriers)
        (Variables|Default|SetTicketActive? false)
        (else
          (Collision|SetCollisionEnabled _cube "QueryAndPhysics"))))))

(event Custom|close%20barriers
  (bind _cube (Variables|Default|GetCube))
  ;[1 1 1] Open and close Gates
  (Variables|Default|SetOpen? false)
  (bind _opentrack (Timeline|OpenBarriers ReverseFromEnd)
    (:Update
      (Transformation|SetRelativeRotation (Variables|Default|GetBarrier_Door) (Math|Rotator|Lerp(Rotator) "0, 0, 0" "0,90.000000, 0" _opentrack) false false)
      (Transformation|SetRelativeRotation (Variables|Default|GetBarrier_Door1) (Math|Rotator|Lerp(Rotator) "0,180.000000, 0" "0,270.000000, 0" _opentrack) false false))
    (:Finished
      (if (Variables|Default|GetOpen?)
        (Collision|SetCollisionEnabled _cube "NoCollision")
        (Utilities|FlowControl|Delay 12.0)
        (CallFunction|CloseBarriers)
        (Variables|Default|SetTicketActive? false)
        (else
          (Collision|SetCollisionEnabled _cube "QueryAndPhysics"))))))

(event EventBeginPlay
  (if (Variables|Default|GetBroken?)
    (Collision|SetCollisionEnabled (Variables|Default|GetCollision) "NoCollision")
    (Transformation|SetRelativeRotation (Variables|Default|GetBarrier_Door) "0,90.000000, 0" false false)
    (Transformation|SetRelativeRotation (Variables|Default|GetBarrier_Door1) "0,270.000000, 0" false false)))

(fn ConstructionScript
  ;[1 1 1] Is the barrier Broken?
  (if (Variables|Default|GetBroken?)
    (Collision|SetCollisionEnabled (Variables|Default|GetCollision) "NoCollision")
    (Transformation|SetRelativeRotation (Variables|Default|GetBarrier_Door) "0,90.000000, 0" false false)
    (Transformation|SetRelativeRotation (Variables|Default|GetBarrier_Door1) "0,270.000000, 0" false false)))