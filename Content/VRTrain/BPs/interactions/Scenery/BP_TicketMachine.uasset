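; A train-scenery ticket machine for VR that dispenses a ticket when a bank card is presented.
; On BeginPlay it copies the EventManager's EN flag and shows an out-of-order widget if broken, otherwise links the buy-ticket widget.
; PurchaseScreen checks WalletManager for an existing ticket, then shows either a notice or a card prompt with arrow and trigger cylinder.
; A BankCard overlapping the armed cylinder spawns the ticket and restores the buy screen.
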(event OnComponentBeginOverlap(Cylinder)
  (params (OverlappedComponent :type Primitive%20Component%20Object%20Reference) (OtherActor :type Actor%20Object%20Reference) (OtherComp :type Primitive%20Component%20Object%20Reference) (OtherBodyIndex :type Integer) (bFromSweep :type Boolean) (SweepResult :type Hit%20Result%20Structure%20%28by%20ref%29))
  ;[1 1 1] Present Card
  (Utilities|Casting|CastToBankCard OtherActor)
  (if (not (and (Variables|Default|GetTicketDispenced?) (Variables|Default|GetBrokenMachine)))
    (if (Variables|Default|GetCanDispence?)
      (bind _returnvalue (Game|SpawnActorfromClass "/Game/VRTrain/BPs/interactions/Ticket.Ticket_C" (Transformation|GetWorldTransform (Variables|Default|GetTicketPoint)) "Undefined" 0 0))
      (Transformation|SetActorRelativeScale3D _returnvalue "0.200000,0.200000,0.200000")
      (Variables|Default|SetTicketDispenced? true)
      (bind _returnvalue_2 (UserInterface|CreateWidget "/Game/VRTrain/BPs/interactions/Widgets/TicketMachine/BuyTicket.BuyTicket_C"))
      (Variables|/Game/VRTrain/BPs/interactions/Widgets/TicketMachine/BuyTicket.BuyTicket_C|SetParent _returnvalue_2 self)
      (UserInterface|SetWidget (Variables|Default|GetWidget) _returnvalue_2)
      (Variables|Default|SetCanDispence? false)
      (Collision|SetCollisionEnabled (Variables|Default|GetCylinder) "NoCollision")
      (Rendering|SetVisibility (Variables|Default|GetSM_Arrow) false false))))

(event Custom|PurchaseScreen
  (bind _outactors (Actor|GetAllActorsOfClass "/Game/VRTrain/BPs/interactions/WalletManager.WalletManager_C"))
  (if (Variables|/Game/VRTrain/BPs/interactions/WalletManager.WalletManager_C|GetTicket? (Utilities|Array|Get(acopy) _outactors))
    (bind _returnvalue (UserInterface|CreateWidget "/Game/VRTrain/BPs/interactions/Widgets/TicketMachine/TicketAlready.TicketAlready_C"))
    (UserInterface|SetWidget (Variables|Default|GetWidget) _returnvalue)
    (else
      (bind _returnvalue_2 (UserInterface|CreateWidget "/Game/VRTrain/BPs/interactions/Widgets/TicketMachine/PresentCard.PresentCard_C"))
      (UserInterface|SetWidget (Variables|Default|GetWidget) _returnvalue_2)
      (Variables|/Game/VRTrain/BPs/interactions/Widgets/TicketMachine/PresentCard.PresentCard_C|SetParent _returnvalue_2 self)
      (Default|UpdateText _returnvalue_2)
      (Collision|SetCollisionEnabled (Variables|Default|GetCylinder) "QueryAndPhysics")
      (Rendering|SetVisibility (Variables|Default|GetSM_Arrow) true false)
      (Variables|Default|SetCanDispence? true))))

(event EventBeginPlay
  ;[1 1 1] Check if out of order
  (|CollapseGraph_0
    (:out
      (|Outorder
        (:else
          (bind _asbuy_ticket (Utilities|Casting|CastToBuyTicket (UserInterface|GetUserWidgetObject (Variables|Default|GetWidget))))
          (Variables|/Game/VRTrain/BPs/interactions/Widgets/TicketMachine/BuyTicket.BuyTicket_C|SetParent _asbuy_ticket self)
          (Collision|SetCollisionEnabled (Variables|Default|GetCylinder) "NoCollision")
          (Rendering|SetVisibility (Variables|Default|GetSM_Arrow) false false))))))

(fn ConstructionScript)