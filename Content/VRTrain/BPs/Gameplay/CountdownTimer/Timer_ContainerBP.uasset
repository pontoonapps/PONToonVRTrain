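; Countdown timer Blueprint for the VR train, tracking minutes and seconds and flagging when the train arrives and leaves.
; Tick feeds a one-second Delay that subtracts NumberAdjuster from Seconds and rolls negative values over into Minutes.
; Reaching the ArrivalTime minute sets TrainArrives; reaching Departime while arrived, or zero, sets TrainLeave and clears TrainArrives.
; DoOnce nodes guard each flag change, and counting stops at zero.
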(event EventTick
  (params (DeltaSeconds :type Float%20%28single-precision%29))
  (if (and (== (Variables|Default|GetMinutes) 0) (== (Variables|Default|GetSeconds) 0))
    (Utilities|FlowControl|DoOnce false
      (:Completed
        (Variables|Default|SetTrainLeave true)
        (Variables|Default|SetTrainArrives false)))
    (else
      (if (Variables|Default|GetTrainArrives)
        (if (and (== (Variables|Default|GetSeconds) 0) (== (Variables|Default|GetMinutes) (Variables|Default|GetDepartime)))
          (Utilities|FlowControl|DoOnce false
            (:Completed
              (Variables|Default|SetTrainLeave true)
              (Variables|Default|SetTrainArrives false))))
        (elif (== (Variables|Default|GetMinutes) (Variables|Default|GetArrivalTime))
          (Utilities|FlowControl|Sequence
            (:then_0
              (Utilities|FlowControl|DoOnce false
                (:Completed
                  (Variables|Default|SetTrainArrives true))))
            (:then_1
              _))))
      (Utilities|FlowControl|Delay 1.0)
      (Variables|Default|SetSeconds (- (Variables|Default|GetSeconds) (Variables|Default|GetNumberAdjuster)))
      (if (< (Variables|Default|GetSeconds) 0)
        (Variables|Default|SetMinutes (- (Variables|Default|GetMinutes) 1))
        (Variables|Default|SetSeconds 59)))))

(fn ConstructionScript)