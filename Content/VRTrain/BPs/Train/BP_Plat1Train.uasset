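; Platform 1 train for a VR game that cycles through arriving, waiting and departing, and can send the player to the "lose" location.
; Timelines slide the mesh between scene points, with a random delay before each arrival and automatic cycling skipped when WinTrainPlatform is set.
; Child BP_EnterTrain arrows reference this actor and are only visible and collidable while the train waits.
; EnterTrain teleports the motion controller pawn to the first "lose"-tagged actor.
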(event Custom|Train%20Arrives
  ;[1 1 1] TrainArrival
  (Variables|Default|SetTrainLoc (Transformation|GetWorldLocation (Variables|Default|GetStaticMesh)))
  (bind _newtrack_0 (Timeline|Timeline_0 PlayFromStart)
    (:Update
      (Variables|Default|Setat%20station? false)
      (Transformation|SetWorldLocation (Variables|Default|GetStaticMesh) (Math|Vector|Lerp(Vector) (Variables|Default|GetTrainLoc) (Transformation|GetWorldLocation (Variables|Default|GetArrivePoint)) _newtrack_0) false false))
    (:Finished
      (Variables|Default|SetCanEnterTrain? true)
      (CallFunction|EnableArrows)
      (Utilities|FlowControl|Delay 3e+01)
      (CallFunction|TrainLeaves))))

(event Custom|TrainLeaves
  ;[1 1 1] Train Leave station
  (Variables|Default|SetTrainLoc (Transformation|GetWorldLocation (Variables|Default|GetStaticMesh)))
  (bind _newtrack_0 (Timeline|Timeline_1 PlayFromStart)
    (:Update
      (CallFunction|DisableArrows)
      (Variables|Default|SetCanEnterTrain? false)
      (Transformation|SetWorldLocation (Variables|Default|GetStaticMesh) (Math|Vector|Lerp(Vector) (Variables|Default|GetTrainLoc) (Transformation|GetWorldLocation (Variables|Default|GetEndPoint)) _newtrack_0) false false))
    (:Finished
      (Variables|Default|Setat%20station? false)
      (Transformation|SetWorldLocation (Variables|Default|GetStaticMesh) (Transformation|GetWorldLocation (Variables|Default|GetStartPoint)) false false)
      (CallFunction|NextTrain))))

(event Custom|EnterTrain
  ;[1 1 1] Enter Train
  (bind _outactors (Actor|GetAllActorswithTag "lose"))
  (bind _asmotion_controller_pawn (Utilities|Casting|CastToMotionControllerPawn (Pawn|GetControlledPawn (Game|GetPlayerController 0))))
  (Transformation|SetActorTransform _asmotion_controller_pawn (Transformation|GetActorTransform (Utilities|Array|Get(acopy) _outactors))))

(event Custom|next%20train
  (Utilities|FlowControl|Delay (Math|Random|RandomFloatinRange 3.0 5e+01))
  (CallFunction|TrainArrives))

(event Custom|DisableArrows
  (bind _exitarray (Variables|Default|GetExitArray))
  (for (_ _array_index) _exitarray
    (bind _asbp_enter_train (Utilities|Casting|CastToBP_EnterTrain (Utilities|Array|Get(acopy) _exitarray _array_index)))
    (Collision|SetCollisionEnabled (Variables|/Game/VRTrain/BPs/interactions/Buttons/BP_EnterTrain.BP_EnterTrain_C|GetCube _asbp_enter_train) "NoCollision")
    (Rendering|SetVisibility (Variables|/Game/VRTrain/BPs/interactions/Buttons/BP_EnterTrain.BP_EnterTrain_C|GetCube _asbp_enter_train) false false)))

(event Custom|EnableArrows
  (bind _exitarray (Variables|Default|GetExitArray))
  (for (_ _array_index) _exitarray
    (bind _asbp_enter_train (Utilities|Casting|CastToBP_EnterTrain (Utilities|Array|Get(acopy) _exitarray _array_index)))
    (Collision|SetCollisionEnabled (Variables|/Game/VRTrain/BPs/interactions/Buttons/BP_EnterTrain.BP_EnterTrain_C|GetCube _asbp_enter_train) "QueryAndPhysics")
    (Rendering|SetVisibility (Variables|/Game/VRTrain/BPs/interactions/Buttons/BP_EnterTrain.BP_EnterTrain_C|GetCube _asbp_enter_train) true false)))

(event EventBeginPlay
  (bind _output_get (Variables|Default|SetExitArray (Utilities|Array|MakeArray (Variables|/Script/Engine.ChildActorComponent|GetChildActor (Variables|Default|GetChildActor9)) (Variables|/Script/Engine.ChildActorComponent|GetChildActor (Variables|Default|GetChildActor10)) (Variables|/Script/Engine.ChildActorComponent|GetChildActor (Variables|Default|GetChildActor2)) (Variables|/Script/Engine.ChildActorComponent|GetChildActor (Variables|Default|GetChildActor3)) (Variables|/Script/Engine.ChildActorComponent|GetChildActor (Variables|Default|GetChildActor11)) (Variables|/Script/Engine.ChildActorComponent|GetChildActor (Variables|Default|GetChildActor4)) (Variables|/Script/Engine.ChildActorComponent|GetChildActor (Variables|Default|GetChildActor5)) (Variables|/Script/Engine.ChildActorComponent|GetChildActor (Variables|Default|GetChildActor6)) (Variables|/Script/Engine.ChildActorComponent|GetChildActor (Variables|Default|GetChildActor7)) (Variables|/Script/Engine.ChildActorComponent|GetChildActor (Variables|Default|GetChildActor8)))))
  (for (_ _array_index) _output_get
    (bind _asbp_enter_train (Utilities|Casting|CastToBP_EnterTrain (Utilities|Array|Get(acopy) _output_get _array_index)))
    (Variables|/Game/VRTrain/BPs/interactions/Buttons/BP_EnterTrain.BP_EnterTrain_C|SetParent _asbp_enter_train self)
    (CallFunction|DisableArrows)
    (if (not (Variables|Default|GetWinTrainPlatform?))
      (Utilities|FlowControl|DoOnce false
        (:Completed
          (Utilities|FlowControl|Delay (Math|Random|RandomFloatinRange 3.0 5e+01))
          (CallFunction|TrainArrives))))))

(fn ConstructionScript)