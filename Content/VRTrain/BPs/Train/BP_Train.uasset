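; BP_Train is a VR train that arrives at and departs from a station, deciding win or lose when the player boards.
; Timelines lerp the train between its start, arrival and end points, with a station sound cue played on arrival and stopped after departure.
; Child BP_EnterTrain arrows get a parent reference and are shown with collision only while the train is stopped.
; Boarding teleports the pawn to the tagged win spot if WinningTrain and WalletManager's Ticket are true, otherwise to lose.
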(event Custom|Train%20Arrives
  ;[1 1 1] TrainArrival
  (Audio|Components|Audio|Play (Variables|Default|GetTrainatStation_Cue) 0.0)
  (Variables|Default|SetTrainLoc (Transformation|GetWorldLocation (Variables|Default|GetTrain)))
  (bind _newtrack_0 (Timeline|Timeline_0 PlayFromStart)
    (:Update
      (Transformation|SetWorldLocation (Variables|Default|GetTrain) (Math|Vector|Lerp(Vector) (Variables|Default|GetTrainLoc) (Transformation|GetWorldLocation (Variables|Default|GetArrivePoint)) _newtrack_0) false false))
    (:Finished
      (Variables|Default|SetCanEnterTrain? true)
      (CallFunction|EnableArrows))))

(event Custom|TrainLeaves
  ;[1 1 1] TrainLeaves
  (Variables|Default|SetTrainLoc (Transformation|GetWorldLocation (Variables|Default|GetArrivePoint)))
  (Variables|Default|SetCanEnterTrain? false)
  (bind _newtrack_0 (Timeline|Timeline_1 PlayFromStart)
    (:Update
      (CallFunction|DiableArrows)
      (Transformation|SetWorldLocation (Variables|Default|GetTrain) (Math|Vector|Lerp(Vector) (Variables|Default|GetTrainLoc) (Transformation|GetWorldLocation (Variables|Default|GetEndPoint)) _newtrack_0) false false))
    (:Finished
      (Audio|Components|Audio|Stop (Variables|Default|GetTrainatStation_Cue)))))

(event Custom|EnterTrain
  (bind _returnvalue (Game|GetPlayerController 0))
  (bind _returnvalue_2 (Pawn|GetControlledPawn _returnvalue))
  (if (Variables|Default|GetWinningTrain?)
    ;[1 1 1] Ticket in wallet?
    (bind _ticket_ (|HasTicket?))
    (if _ticket_
      ;[1 1 1] Win
      (bind _outactors (Actor|GetAllActorswithTag "win"))
      (bind _asmotion_controller_pawn (Utilities|Casting|CastToMotionControllerPawn _returnvalue_2))
      (Transformation|SetActorTransform _asmotion_controller_pawn (Transformation|GetActorTransform (Utilities|Array|Get(acopy) _outactors)))
      (else
        ;[1 1 1] Lose
        (bind _outactors_2 (Actor|GetAllActorswithTag "lose" :!label _label))
        (bind _asmotion_controller_pawn_2 (Utilities|Casting|CastToMotionControllerPawn _returnvalue_2))
        (Transformation|SetActorTransform _asmotion_controller_pawn_2 (Transformation|GetActorTransform (Utilities|Array|Get(acopy) _outactors_2)))))
    (else
      (goto _label))))

(event Custom|diableArrows
  (bind _enterobj (Variables|Default|GetEnterObj))
  (for (_ _array_index) _enterobj
    (bind _asbp_enter_train (Utilities|Casting|CastToBP_EnterTrain (Utilities|Array|Get(acopy) _enterobj _array_index)))
    (Collision|SetCollisionEnabled (Variables|/Game/VRTrain/BPs/interactions/Buttons/BP_EnterTrain.BP_EnterTrain_C|GetCube _asbp_enter_train) "NoCollision")
    (Rendering|SetVisibility (Variables|/Game/VRTrain/BPs/interactions/Buttons/BP_EnterTrain.BP_EnterTrain_C|GetCube _asbp_enter_train) false false)))

(event Custom|EnableArrows
  (bind _enterobj (Variables|Default|GetEnterObj))
  (for (_ _array_index) _enterobj
    (bind _asbp_enter_train (Utilities|Casting|CastToBP_EnterTrain (Utilities|Array|Get(acopy) _enterobj _array_index)))
    (Collision|SetCollisionEnabled (Variables|/Game/VRTrain/BPs/interactions/Buttons/BP_EnterTrain.BP_EnterTrain_C|GetCube _asbp_enter_train) "QueryAndPhysics")
    (Rendering|SetVisibility (Variables|/Game/VRTrain/BPs/interactions/Buttons/BP_EnterTrain.BP_EnterTrain_C|GetCube _asbp_enter_train) true false)))

(event EventBeginPlay
  (bind _output_get (Variables|Default|SetEnterObj (Utilities|Array|MakeArray (Variables|/Script/Engine.ChildActorComponent|GetChildActor (Variables|Default|GetChildActor1)) (Variables|/Script/Engine.ChildActorComponent|GetChildActor (Variables|Default|GetChildActor)) (Variables|/Script/Engine.ChildActorComponent|GetChildActor (Variables|Default|GetChildActor9)) (Variables|/Script/Engine.ChildActorComponent|GetChildActor (Variables|Default|GetChildActor3)) (Variables|/Script/Engine.ChildActorComponent|GetChildActor (Variables|Default|GetChildActor4)) (Variables|/Script/Engine.ChildActorComponent|GetChildActor (Variables|Default|GetChildActor5)) (Variables|/Script/Engine.ChildActorComponent|GetChildActor (Variables|Default|GetChildActor6)) (Variables|/Script/Engine.ChildActorComponent|GetChildActor (Variables|Default|GetChildActor7)) (Variables|/Script/Engine.ChildActorComponent|GetChildActor (Variables|Default|GetChildActor8)) (Variables|/Script/Engine.ChildActorComponent|GetChildActor (Variables|Default|GetChildActor2)) (Variables|/Script/Engine.ChildActorComponent|GetChildActor (Variables|Default|GetChildActor10)) (Variables|/Script/Engine.ChildActorComponent|GetChildActor (Variables|Default|GetChildActor11)) (Variables|/Script/Engine.ChildActorComponent|GetChildActor (Variables|Default|GetChildActor12)) (Variables|/Script/Engine.ChildActorComponent|GetChildActor (Variables|Default|GetChildActor13)) (Variables|/Script/Engine.ChildActorComponent|GetChildActor (Variables|Default|GetChildActor14)) (Variables|/Script/Engine.ChildActorComponent|GetChildActor (Variables|Default|GetChildActor15)))))
  (for (_ _array_index) _output_get
    (bind _asbp_enter_train (Utilities|Casting|CastToBP_EnterTrain (Utilities|Array|Get(acopy) _output_get _array_index)))
    (Variables|/Game/VRTrain/BPs/interactions/Buttons/BP_EnterTrain.BP_EnterTrain_C|SetParent _asbp_enter_train self)
    (CallFunction|DiableArrows)))

(fn ConstructionScript)